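; BP_RippleOperator relays particle positions from the GPUWaterDrips Niagara system into MPC_RipplePositions, apparently to drive material water ripples.
; On BeginPlay it registers itself as the system's BP_CallBack object to receive exported particle data.
; Each particle's position and the current game time are packed into a "drop"-indexed vector parameter.
; A wrapping cursor treats the 16 parameters as a ring buffer, overwriting the oldest drops.
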(event EventBeginPlay
  (Class|NiagaraComponent|SetVariableObject (Variables|Default|GetGPUWaterDrips) "BP_CallBack" self))

(event EventParticleData
  (params (Data :type Array%20of%20Basic%20Particle%20Data%20Structures) (NiagaraSystem :type Niagara%20System%20Object%20Reference) (SimulationPositionOffset :type Vector%20%28by%20ref%29 :default "0, 0, 0"))
  (for _array_element Data
    (Rendering|Material|SetVectorParameterValue "/Game/CustomRenderInfo/MPC_RipplePositions.MPC_RipplePositions" (Utilities|String|StringToName (Utilities|String|Append "drop" (Utilities|String|ToString(Integer) (Variables|Default|GetcursorIndex)))) (Math|Color|MakeColor (.X (Math|Vector|BreakVector (.Position (Utilities|Struct|BreakBasicParticleData _array_element)))) (.Y (Math|Vector|BreakVector (.Position (Utilities|Struct|BreakBasicParticleData _array_element)))) (.Z (Math|Vector|BreakVector (.Position (Utilities|Struct|BreakBasicParticleData _array_element)))) (Utilities|Time|GetTimeSeconds)) :!class /Script/Engine.KismetMaterialLibrary)
    (bind _result (Math|Integer|IncrementInt (Variables|Default|GetcursorIndex))
      (:%20%20
        (if (== _result 16)
          (Variables|Default|SetcursorIndex 0) ; renew the cursor
        )))))

(fn ConstructionScript)